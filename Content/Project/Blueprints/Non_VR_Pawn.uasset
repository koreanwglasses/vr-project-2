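; Non-VR pawn that lets the player pick up, roll and drop objects with mouse and keyboard.
; Left mouse press line-traces forward from AttachTarget and hands that component to any hit actor implementing PickupActorInterface; release tells the held actor to drop.
; Holding X or Z sets a signed roll speed that Tick applies to AttachTarget as frame-rate-independent local rotation.
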(event Custom|PickUpObject
  (bind _attachtarget (Variables|Default|GetAttachTarget))
  (bind _returnvalue (Transformation|GetWorldLocation _attachtarget))
  (bind (_outhit _returnvalue_2) (Collision|LineTraceForObjects _returnvalue (+ _returnvalue (* (Math|Vector|GetForwardVector _attachtarget) 1e+03)) (Utilities|Array|MakeArray "ObjectTypeQuery2" "ObjectTypeQuery4") false 0 "ForDuration"))
  (if _returnvalue_2
    (if (Utilities|DoesObjectImplementInterface (.HitActor (Collision|BreakHitResult _outhit)) "/Game/VirtualRealityBP/Blueprints/PickupActorInterface.PickupActorInterface_C")
      (bind _aspickup_actor_interface (Utilities|Casting|CastToPickupActorInterface (.HitActor (Collision|BreakHitResult _outhit))))
      (bind _output_get (Variables|Default|SetPickedUpActor _aspickup_actor_interface))
      (Class|PickupActorInterface|Pickup(Message) (Utilities|ToObject(Interface) _output_get) (Variables|Default|GetAttachTarget))
      (Variables|Default|SetIsHoldingObject true))))

(event Custom|DropObject
  (Utilities|IsValid (Utilities|ToObject(Interface) (Variables|Default|GetPickedUpActor))
    (:Is%20Valid
      (Default|Drop (Variables|Default|GetPickedUpActor))
      (Variables|Default|SetIsHoldingObject false)
      (Variables|Default|SetPickedUpActor 0))))

(event EventBeginPlay)

(event Collision|EventActorBeginOverlap
  (params (OtherActor :type Actor%20Object%20Reference)))

(event EventTick
  (params (DeltaSeconds :type Float%20%28single-precision%29))
  (bind _rollspeed (Variables|Default|GetRollSpeed))
  (if (!= _rollspeed 0.0)
    (Transformation|AddLocalRotation (Variables|Default|GetAttachTarget) (Math|Rotator|MakeRotator (* DeltaSeconds _rollspeed) 0.0 0.0) false false)))

(event Input|MouseEvents|LeftMouseButton
  (params (Key :type Key%20Structure :default "None"))
  (:Pressed
    (CallFunction|PickUpObject))
  (:Released
    (CallFunction|DropObject)))

(event Input|KeyboardEvents|X
  (params (Key :type Key%20Structure :default "None"))
  (:Pressed
    (Variables|Default|SetRollSpeed 1.5e+02))
  (:Released
    (Variables|Default|SetRollSpeed 0.0)))

(event Input|KeyboardEvents|Z
  (params (Key :type Key%20Structure :default "None"))
  (:Pressed
    (Variables|Default|SetRollSpeed -1.5e+02))
  (:Released
    (Variables|Default|SetRollSpeed 0.0)))

(fn ConstructionScript)