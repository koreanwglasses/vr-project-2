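; A VR pickup cup whose glow toggles each time BP_MotionController grabs it.
; Pickup disables physics, attaches the root to the given component keeping world transform, then flips IsOn to set the light's visibility and swap the mesh material between glowing and plain glass.
; Drop re-enables physics simulation and detaches the actor in place.
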(event EventBeginPlay)

(event Collision|EventActorBeginOverlap
  (params (OtherActor :type Actor%20Object%20Reference)))

(event EventTick
  (params (DeltaSeconds :type Float%20%28single-precision%29)))

(event EventPickup
  (params (AttachTo :type Scene%20Component%20Object%20Reference))
  (bind _staticmeshcomponent (Variables|Debug|GetStaticMeshComponent))
  (Physics|SetSimulatePhysics (Variables|Debug|GetStaticMeshComponent) false)
  (Transformation|AttachComponentToComponent (VehicleSound|GetRootComponent) AttachTo "None" "KeepWorld" "KeepWorld" "KeepWorld" false)
  (bind _output_get (Variables|Default|SetIsOn (not (Variables|Default|GetIsOn))))
  (Utilities|FlowControl|Sequence
    (:then_0
      (Rendering|SetVisibility (Variables|Default|GetLight) _output_get false))
    (:then_1
      (if _output_get
        (Rendering|Material|SetMaterial _staticmeshcomponent 0 "/Game/Project/Materials/Glow_Glass.Glow_Glass")
        (else
          (Rendering|Material|SetMaterial _staticmeshcomponent 0 "/Game/Project/Materials/Glass.Glass"))))))

(event EventDrop
  (Physics|SetSimulatePhysics (Variables|Debug|GetStaticMeshComponent) true)
  (Transformation|DetachFromActor "KeepWorld" "KeepWorld" "KeepWorld"))

(fn ConstructionScript)