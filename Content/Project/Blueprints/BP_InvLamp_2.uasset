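; BP_InvLamp_2 is a lamp that motion controllers can pick up, toggling its light on each pickup.
; Pickup disables physics and attaches the lamp to the controller, then flips IsOn to drive the PointLight, the lampshade material and the root visibility of a referenced Sun actor.
; Drop re-enables physics and detaches the lamp, leaving its on/off state unchanged.
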(event EventBeginPlay)

(event Collision|EventActorBeginOverlap
  (params (OtherActor :type Actor%20Object%20Reference)))

(event EventTick
  (params (DeltaSeconds :type Float%20%28single-precision%29)))

(event EventPickup
  (params (AttachTo :type Scene%20Component%20Object%20Reference))
  (bind _lamp_pcube7 (Variables|Default|GetLamp_pCube7))
  (Utilities|FlowControl|Sequence
    (:then_0
      (Physics|SetSimulatePhysics (Variables|Debug|GetStaticMeshComponent) false)
      (Transformation|AttachComponentToComponent (VehicleSound|GetRootComponent) AttachTo "None" "KeepWorld" "KeepWorld" "KeepWorld" false))
    (:then_1
      (bind _output_get (Variables|Default|SetIsOn (not (Variables|Default|GetIsOn))))
      (Utilities|FlowControl|Sequence
        (:then_0
          (Rendering|SetVisibility (Variables|Default|GetPointLight) _output_get true))
        (:then_1
          (if _output_get
            (Rendering|Material|SetMaterial _lamp_pcube7 0 "/Game/Project/Materials/Lampshade_On.Lampshade_On")
            (else
              (Rendering|Material|SetMaterial _lamp_pcube7 0 "/Game/Project/Materials/Lampshade_Off.Lampshade_Off"))))
        (:then_2
          (Rendering|SetVisibility (Variables|/Script/Engine.Actor|GetRootComponent (Variables|Default|GetSun)) _output_get false))))))

(event EventDrop
  (Physics|SetSimulatePhysics (Variables|Debug|GetStaticMeshComponent) true)
  (Transformation|DetachFromActor "KeepWorld" "KeepWorld" "KeepWorld"))

(fn ConstructionScript)